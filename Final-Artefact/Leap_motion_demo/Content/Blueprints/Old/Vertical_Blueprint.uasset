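; Actor Blueprint in an Old folder that moves a static mesh vertically based on hand movement, apparently from Leap Motion tracking.
; Tick samples wrist Z before and after a short Delay, printing both, and calls MoveUp or MoveDown on the difference.
; Each plays a timeline that lerps the mesh from the latest wrist position, not its own location, toward a fixed offset above or below its location.
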(event `MoveUp`
  (set `self.Up Scale` (+ (`SceneComponent.K2_GetComponentLocation` (`self.StaticMeshComponent`)) (0.0 0.0 10.0)))
  (bind (_direction _moveup) (`Timeline|Up`)
    (:`Update`
      (`SceneComponent.K2_SetWorldLocation` (`self.StaticMeshComponent`) (`KismetMathLibrary.VLerp` (`self.NewPos`) (`self.Up Scale`) _moveup) false false))))

(event `self.ReceiveBeginPlay`
  (`self.EnableInput` (`GameplayStatics.GetPlayerController` 0) null))

(event `self.ReceiveTick`
  (params (DeltaSeconds :type "Float (single-precision)"))
  (bind _wristposition (`LeapArm.WristPosition` (`LeapHand.Arm` (stale `LeapEventInterface.LeapRightHandMoved` hand))))
  (bind _output_get (set `self.InitialPos` _wristposition))
  (bind _output_get_2 (set `self.InitialFloat` (.z _output_get)))
  (`KismetSystemLibrary.PrintString` (`KismetStringLibrary.Conv_DoubleToString` _output_get_2))
  (`KismetSystemLibrary.Delay` 0.09)
  (bind _output_get_3 (set `self.NewPos` _wristposition))
  (bind _output_get_4 (set `self.NewFloat` (.z _output_get_3)))
  (`KismetSystemLibrary.PrintString` (`KismetStringLibrary.Conv_DoubleToString` _output_get_4) true true (struct :`R` 1.0 :`G` 0.704199 :`A` 1.0))
  (if (> (`self.NewFloat`) (`self.InitialFloat`))
    (`self.MoveUp`)
    (elif (< (`self.NewFloat`) (`self.InitialFloat`))
      (`self.MoveDown`))))

(event `LeapEventInterface.LeapLeftHandMoved`
  (params (hand :type "LeapHand Object Reference")))

(event `LeapEventInterface.LeapRightHandMoved`
  (params (hand :type "LeapHand Object Reference")))

(event `MoveDown`
  (set `self.DownScale` (- (`SceneComponent.K2_GetComponentLocation` (`self.StaticMeshComponent`)) (0.0 0.0 10.0)))
  (bind (_direction _movedown) (`Timeline|Down`)
    (:`Update`
      (`SceneComponent.K2_SetWorldLocation` (`self.StaticMeshComponent`) (`KismetMathLibrary.VLerp` (`self.NewPos`) (`self.DownScale`) _movedown) false false))))

(fn `UserConstructionScript`)