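; Player-one Blueprint that moves its static mesh (a plate, per the comments) using Leap Motion right-hand input.
; Tick truncates the hand's wrist X/Y, calls Movement and debug-prints a wrist-derived rotation.
; Movement compares current to previous X/Y in sequence, calling short eased MoveComponentTo steps by MovScale from actor location.
; PreviousX and PreviousY are never updated in this graph.
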(event `LeapEventInterface.LeapRightHandMoved`
  (params (hand :type "LeapHand Object Reference"))
  ;[1 1 1] Detect hand
  ;;[1 0.4735 0.8308] One movement is detected from the players right hand, the X and Y values are then promoted to varables (to calculate player hand movement)
)

(event `self.ReceiveTick`
  (params (DeltaSeconds :type "Float (single-precision)"))
  ;[1 1 1] Detect hand
  ;;[1 0.4735 0.8308] The follwoing tick, constantly updates the aformentioned promoted variables (for more accurate raw input data readings)
  (bind _wristposition (`LeapArm.WristPosition` (`LeapHand.Arm` (stale `LeapEventInterface.LeapRightHandMoved` hand))))
  (set `self.CurrentX` (`KismetMathLibrary.FTrunc` (.x _wristposition)))
  (set `self.CurrentY` (`KismetMathLibrary.FTrunc` (.y _wristposition)))
  ;[1 0.4735 0.8308] The movement function will apply the movement to the players desired direction and speed, the function is called in the tick to initialse the listeners that detect the players direction ( X and Y values)
  (`self.Movement `)
  ;[0 0 0] Debug
  (`KismetSystemLibrary.PrintString` (`KismetStringLibrary.Conv_RotatorToString` (`KismetMathLibrary.MakeRotationFromAxes` _wristposition _wristposition _wristposition)) true true (struct :`R` 1.0 :`B` 0.047119 :`A` 1.0) 5.0))

(event `Movement`
  ;[1 1 1] Comment
  ;;[1 0.1812 0.3813] The sequence sets the order in which the listeners check to see moevement direction and distance between the current and previpus axis values
  (`|ExecutionSequence`
    (:`then_0`
      ;;[1 0.1812 0.3813] Here the axis values distance are compared in order to detect the direction in which the players input will be directed
      (if (> (`self.CurrentX`) (`self.PreviousX`))
        ;;[1 0.1812 0.3813] Here the movement input is added to plates
        (`KismetSystemLibrary.MoveComponentTo` (`self.StaticMeshComponent`) (+ (`self.K2_GetActorLocation`) (`KismetMathLibrary.MakeVector` (`self.MovScale`))) (`SceneComponent.K2_GetComponentRotation` (`self.StaticMeshComponent`)) true true 0.02)))
    (:`then_1`
      (if (> (`self.PreviousX`) (`self.CurrentX`))
        (`KismetSystemLibrary.MoveComponentTo` (`self.StaticMeshComponent`) (- (`self.K2_GetActorLocation`) (`KismetMathLibrary.MakeVector` (`self.MovScale`))) (`SceneComponent.K2_GetComponentRotation` (`self.StaticMeshComponent`)) true true 0.02)))
    (:`then_2`
      (if (> (`self.CurrentY`) (`self.PreviousY`))
        (`KismetSystemLibrary.MoveComponentTo` (`self.StaticMeshComponent`) (+ (`self.K2_GetActorLocation`) (`KismetMathLibrary.MakeVector` 0.0 (`self.MovScale`))) (`SceneComponent.K2_GetComponentRotation` (`self.StaticMeshComponent`)) true true 0.02)))
    (:`then_3`
      (if (> (`self.PreviousY`) (`self.CurrentY`))
        (`KismetSystemLibrary.MoveComponentTo` (`self.StaticMeshComponent`) (- (`self.K2_GetActorLocation`) (`KismetMathLibrary.MakeVector` 0.0 (`self.MovScale`))) (`SceneComponent.K2_GetComponentRotation` (`self.StaticMeshComponent`)) true true 0.02)))))

(fn `UserConstructionScript`)