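; Player one Blueprint, apparently an older prototype, that moves a static mesh cube up or down with a Leap Motion right hand.
; Each Tick compares wrist height to PreviousPos, then eases the mesh a fixed step along Z via MoveComponentTo.
; PreviousPos is never updated and the direction flags are never cleared here.
; InitialPos and CubeZ are written but drive nothing, and GeneratePlayerCube is an empty stub.
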(event `Check hand movement`
  (bind _staticmeshcomponent (`self.StaticMeshComponent`))
  (bind _curentpos (`self.CurentPos`))
  (bind _previouspos (`self.PreviousPos`))
  (bind _staticmeshcomponent_2 (`self.StaticMeshComponent`))
  ;[1 1 1] Event that checks if the hand if moving and returns if it is moving up or down
  (if (== (`self.CurentPos`) 0.0)
    _
    (elif (> _curentpos _previouspos)
      (set `self.Hand moving up ` true)
      (set `self.Cube Z` (- _curentpos _previouspos))
      (`KismetSystemLibrary.MoveComponentTo` _staticmeshcomponent_2 (+ (`SceneComponent.K2_GetComponentLocation` _staticmeshcomponent_2) (0.0 0.0 10.0)) (`SceneComponent.K2_GetComponentRotation` _staticmeshcomponent_2) true true 0.02)
      (elif (< (`self.CurentPos`) _previouspos)
        (set `self.Hand moving down` true)
        (set `self.Cube Z` (- _curentpos _previouspos))
        (`KismetSystemLibrary.MoveComponentTo` _staticmeshcomponent (- (`SceneComponent.K2_GetComponentLocation` _staticmeshcomponent) (0.0 0.0 10.0)) (`SceneComponent.K2_GetComponentRotation` _staticmeshcomponent) true true 0.02)))))

(event `self.ReceiveBeginPlay`
  ;[1 1 1] Initialise
  (set `self.InitialPos` (.z (`LeapArm.WristPosition` (`LeapHand.Arm` (stale `LeapEventInterface.LeapRightHandMoved` hand)))))
  (`self.EnableInput` (`GameplayStatics.GetPlayerController` 0))
  (`self.SetActorEnableCollision` true))

(event `LeapEventInterface.LeapRightHandMoved`
  (params (hand :type "LeapHand Object Reference"))
  ;[1 1 1] Initialise
  (`KismetSystemLibrary.PrintString` (`KismetStringLibrary.Conv_DoubleToString` (.z (`LeapArm.WristPosition` (`LeapHand.Arm` hand)))))
  (set `self.Cube Z` (.z (`SceneComponent.K2_GetComponentLocation` (`self.StaticMeshComponent`)))))

(event `self.ReceiveTick`
  (params (DeltaSeconds :type "Float (single-precision)"))
  ;[1 1 1] Initialise
  (set `self.CurentPos` (.z (`LeapArm.WristPosition` (`LeapHand.Arm` (stale `LeapEventInterface.LeapRightHandMoved` hand)))))
  (`self.Check hand movement`))

(fn `Generate player cube`
  (params (Radius :type "Float (double-precision)") (Location :type "Vector Structure")))

(fn `UserConstructionScript`)