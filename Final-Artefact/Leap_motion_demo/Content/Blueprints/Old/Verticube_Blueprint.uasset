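; Verticube actor that moves vertically under keyboard or Leap Motion control.
; W or right grab sets a target height 10 units above the mesh's current Z, S or left grab 10 below.
; Tick snaps the actor to that height without sweep.
; Circle gestures only print; right-hand wrist sampling prints and stores positions, but its height calculation and the Timeline lerp smoothing are left unconnected.
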(event `self.ReceiveBeginPlay`
  (`self.EnableInput` (`GameplayStatics.GetPlayerController` 0))
  (`LeapController.EnableGesture` (`self.LeapController`) "GESTURE_TYPE_CIRCLE" true))

(event `self.ReceiveTick`
  (params (DeltaSeconds :type "Float (single-precision)"))
  (bind _output_get (set `self.OldLocal` (`SceneComponent.K2_GetComponentLocation` (`self.StaticMeshComponent`))))
  (set `self.MidPos` _output_get)
  (set `self.HandLocal` (.z (`self.MidPos`)))
  (set `self.NewLocal` (`KismetMathLibrary.MakeVector` (.x (`self.MidPos`)) (.y (`self.MidPos`)) (`self.NewHLocal`)))
  (`self.K2_SetActorLocation` (`self.NewLocal`)))

(event `Key|W`
  (params (Key :type "Key Structure"))
  (:`Pressed`
    (set `self.NewHLocal` (+ (`self.HandLocal`) 10.0) :!label _label)))

(event `Key|LeapRightGrab`
  (params (Key :type "Key Structure"))
  (:`Pressed`
    (`KismetSystemLibrary.PrintString` "Hello" true true (struct :`G` 1.0 :`B` 0.268722 :`A` 1.0))
    (goto _label)))

(event `LeapEventInterface.GestureDetected`
  (params (gesture :type "LeapGesture Object Reference"))
  (switch `LeapGestureType` "GESTURE_TYPE_CIRCLE"
    (:`GESTURE_TYPE_CIRCLE`
      (`KismetSystemLibrary.PrintString` "Circle" true true (struct :`R` 1.0 :`G` 0.334474 :`B` 0.889962 :`A` 1.0) 1e-16))))

(event `Key|S`
  (params (Key :type "Key Structure"))
  (:`Pressed`
    (set `self.NewHLocal` (- (`self.HandLocal`) 10.0) :!label _label_2)))

(event `Key|LeapLeftGrab`
  (params (Key :type "Key Structure"))
  (:`Pressed`
    (goto _label_2)))

(event `LeapEventInterface.LeapRightHandMoved`
  (params (hand :type "LeapHand Object Reference"))
  (bind _wristposition (`LeapArm.WristPosition` (`LeapHand.Arm` hand)))
  (`KismetSystemLibrary.PrintString` "Magic Activated" true true (struct :`G` 0.66 :`B` 1.0 :`A` 1.0) 1e-24)
  (set `self.HandOld` _wristposition)
  (`KismetSystemLibrary.Delay` 0.2)
  (set `self.HandNew` _wristposition))

(fn `UserConstructionScript`)