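; Player-one actor Blueprint that steers its static mesh with the right hand through Leap Motion.
; Tick truncates the tracked wrist's X and Y, then calls Movement to compare them with PreviousX and PreviousY.
; Each difference triggers a short eased MoveComponentTo, targeting the actor's location offset by MovScale on that axis.
; The graph never updates the Previous values, so comparisons use their stored values.
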(event `self.ReceiveBeginPlay`
  (`self.EnableInput` null))

(event `LeapEventInterface.LeapRightHandMoved`
  (params (hand :type "LeapHand Object Reference"))
  ;[1 1 1] Detect hand
)

(event `self.ReceiveTick`
  (params (DeltaSeconds :type "Float (single-precision)"))
  ;[1 1 1] Detect hand
  (set `self.CurrentX` (`KismetMathLibrary.FTrunc` (.x (`LeapArm.WristPosition` (`LeapHand.Arm` (stale `LeapEventInterface.LeapRightHandMoved` hand))))))
  (set `self.CurrentY` (`KismetMathLibrary.FTrunc` (.y (`LeapArm.WristPosition` (`LeapHand.Arm` (stale `LeapEventInterface.LeapRightHandMoved` hand))))))
  (`self.Movement `))

(event `Movement`
  (`|ExecutionSequence`
    (:`then_0`
      (if (> (`self.CurrentX`) (`self.PreviousX`))
        (`KismetSystemLibrary.MoveComponentTo` (`self.StaticMeshComponent`) (+ (`self.K2_GetActorLocation`) (`KismetMathLibrary.MakeVector` (`self.MovScale`))) (`SceneComponent.K2_GetComponentRotation` (`self.StaticMeshComponent`)) true true 0.02)))
    (:`then_1`
      (if (> (`self.PreviousX`) (`self.CurrentX`))
        (`KismetSystemLibrary.MoveComponentTo` (`self.StaticMeshComponent`) (- (`self.K2_GetActorLocation`) (`KismetMathLibrary.MakeVector` (`self.MovScale`))) (`SceneComponent.K2_GetComponentRotation` (`self.StaticMeshComponent`)) true true 0.02)))
    (:`then_2`
      (if (> (`self.CurrentY`) (`self.PreviousY`))
        (`KismetSystemLibrary.MoveComponentTo` (`self.StaticMeshComponent`) (+ (`self.K2_GetActorLocation`) (`KismetMathLibrary.MakeVector` 0.0 (`self.MovScale`))) (`SceneComponent.K2_GetComponentRotation` (`self.StaticMeshComponent`)) true true 0.02)))
    (:`then_3`
      (if (> (`self.PreviousY`) (`self.CurrentY`))
        (`KismetSystemLibrary.MoveComponentTo` (`self.StaticMeshComponent`) (- (`self.K2_GetActorLocation`) (`KismetMathLibrary.MakeVector` 0.0 (`self.MovScale`))) (`SceneComponent.K2_GetComponentRotation` (`self.StaticMeshComponent`)) true true 0.02)))))

(fn `UserConstructionScript`)