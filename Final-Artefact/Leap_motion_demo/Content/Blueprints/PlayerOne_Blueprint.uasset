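; Player one Blueprint that moves a static mesh cube vertically from Leap Motion hand wrist height.
; Tick reads wrist Z, compares it to PreviousPos to flag up or down movement, then moves the mesh by the CubeZ difference.
; PreviousPos is never updated here, and the right-hand-moved event overwrites CubeZ with the mesh's world Z.
; The target relative location is built from world location; GeneratePlayerCube is an empty stub.
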(event `LeapEventInterface.LeapRightHandMoved`
  (params (hand :type "LeapHand Object Reference"))
  (set `self.Cube Z` (.z (`SceneComponent.K2_GetComponentLocation` (`self.StaticMeshComponent`)))))

(event `self.ReceiveBeginPlay`
  (set `self.InitialPos` (.z (`LeapArm.WristPosition` (`LeapHand.Arm` (stale `LeapEventInterface.LeapRightHandMoved` hand))))))

(event `Check hand movement`
  (bind _curentpos (`self.CurentPos`))
  (bind _previouspos (`self.PreviousPos`))
  ;[1 1 1] Event that checks if the hand if moving and returns if it is moving up or down
  (if (== (`self.CurentPos`) 0.0)
    _
    (elif (`self.Hand is still`)
      _
      (elif (> _curentpos _previouspos)
        (set `self.Hand moving up ` true)
        (set `self.Cube Z` (- _curentpos _previouspos))
        (`KismetSystemLibrary.PrintString` "moving up" true true (struct :`R` 1.0 :`A` 1.0) 0.2)
        (elif (< (`self.CurentPos`) _previouspos)
          (set `self.Hand moving down` true)
          (set `self.Cube Z` (- _curentpos _previouspos))
          (`KismetSystemLibrary.PrintString` "moving down" true true (struct :`G` 0.66 :`B` 1.0 :`A` 1.0) 0.2))))))

(event `self.ReceiveTick`
  (params (DeltaSeconds :type "Float (single-precision)"))
  (bind _staticmeshcomponent (`self.StaticMeshComponent`))
  (set `self.CurentPos` (.z (`LeapArm.WristPosition` (`LeapHand.Arm` (stale `LeapEventInterface.LeapRightHandMoved` hand)))))
  (`self.Check hand movement`)
  (`KismetSystemLibrary.MoveComponentTo` _staticmeshcomponent (+ (`SceneComponent.K2_GetComponentLocation` _staticmeshcomponent) (`KismetMathLibrary.MakeVector` 0.0 0.0 (`self.Cube Z`)))))

(fn `Generate player cube`
  (params (Radius :type "Float (double-precision)") (Location :type "Vector Structure")))

(fn `UserConstructionScript`)