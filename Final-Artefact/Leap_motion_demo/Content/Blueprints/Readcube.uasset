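; Readcube is an unfinished Leap Motion experiment to move a cube vertically with the right hand's wrist height.
; All events, including hand-moved, movement check, Tick and MoveUp input, are empty, so none of the logic runs.
; Disconnected fragments compare current and previous wrist Z to flag up or down motion and derive an offset for MoveComponentTo.
; Another unwired fragment applies vertical movement input from an axis value.
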(event `LeapEventInterface.LeapRightHandMoved`
  (params (hand :type "LeapHand Object Reference")))

(event `self.ReceiveBeginPlay`)

(event `Check hand movement`
  ;[1 1 1] Event that checks if the hand if moving and returns if it is moving up or down
)

(event `self.ReceiveTick`
  (params (DeltaSeconds :type "Float (single-precision)")))

(event `InputAxis|MoveUp`
  (params (AxisValue :type "Float (single-precision)")))

(fn `UserConstructionScript`)